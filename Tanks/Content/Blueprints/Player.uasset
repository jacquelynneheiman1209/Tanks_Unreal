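; Player pawn Blueprint that handles Enhanced Input movement and turning.
; On possession by a player controller, it adds the IMC_ThirdPerson_Player mapping context.
; The rotate action yaws the actor by input, rotation speed and frame time.
; The move action applies an unswept, unit-length forward offset, with input, speed and frame time added to the yaw angle rather than scaling the distance.
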(event `self.ReceivePossessed`
  (params (NewController :type "Controller Object Reference"))
  (bind _asplayer_controller (cast `PlayerController` NewController))
  (`EnhancedInputSubsystemInterface.AddMappingContext` (pcsubsystem `EnhancedInputLocalPlayerSubsystem` _asplayer_controller) "/Game/Input/IMC_ThirdPerson_Player.IMC_ThirdPerson_Player" 0 (struct)))

(event `EnhancedInput|/Game/Input/IA_MoveForward_Player`
  (params (ActionValue :type "Float (double-precision)") (ElapsedSeconds :type "Float (double-precision)") (TriggeredSeconds :type "Float (double-precision)") (InputAction :type "InputAction Object Reference" :default "/Game/Input/IA_MoveForward_Player.IA_MoveForward_Player"))
  (:`Triggered`
    (`self.K2_AddActorWorldOffset` (`KismetMathLibrary.GetForwardVector` (`KismetMathLibrary.MakeRotator` 0.0 0.0 (+ (* ActionValue (`self.MoveSpeed`) (`GameplayStatics.GetWorldDeltaSeconds`)) (.yaw (`self.K2_GetActorRotation`))))))))

(event `EnhancedInput|/Game/Input/IA_RotateLeft_Player`
  (params (ActionValue :type "Float (double-precision)") (ElapsedSeconds :type "Float (double-precision)") (TriggeredSeconds :type "Float (double-precision)") (InputAction :type "InputAction Object Reference" :default "/Game/Input/IA_RotateLeft_Player.IA_RotateLeft_Player"))
  (:`Triggered`
    (`self.K2_AddActorWorldRotation` (`KismetMathLibrary.MakeRotator` 0.0 0.0 (* ActionValue (`self.RotationSpeped`) (`GameplayStatics.GetWorldDeltaSeconds`))))))

(fn `UserConstructionScript`)